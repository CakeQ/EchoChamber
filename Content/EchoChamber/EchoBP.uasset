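; EchoBP is an actor that acts as an expanding echo, growing a sphere collider outward and drawing it as a debug circle.
; Each Tick increases EchoRadius in proportion to its current value and delta time, giving exponential growth, then resizes EchoCollider with overlap updates.
; The ring uses debug drawing with variable segments, color and thickness; actor overlaps only trigger a debug sphere draw with no inputs set.
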(event EventBeginPlay)

(event Collision|EventActorBeginOverlap
  (params (OtherActor :type Actor%20Object%20Reference))
  (Rendering|Debug|DrawDebugSphere "0, 0, 0" 1e+02 12 "(R=1.000000,G=1.000000,B=1.000000,A=1.000000)" 0.0))

(event EventTick
  (params (DeltaSeconds :type Float%20%28single-precision%29))
  (bind _output_get (Variables|Default|SetEchoRadius (+ (* DeltaSeconds (Variables|Default|GetEchoRadius)) (Variables|Default|GetEchoRadius))))
  (Components|Sphere|SetSphereRadius (Variables|Default|GetEchoCollider) _output_get true)
  (Rendering|Debug|DrawDebugCircle (Transformation|GetActorLocation) _output_get (Variables|Default|GetEchoSegments) (Math|Conversions|ToLinearColor(Color) (Variables|Default|GetEchoColor)) 0.0 (Variables|Default|GetEchoThickness) "0.000000,1.000000,0.000000" "0.000000,0.000000,1.000000"))

(fn ConstructionScript)